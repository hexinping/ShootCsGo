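; Water projectile that cools and wets what it hits through an elemental damage interface.
; On spawn it launches along its rotation with a fire sound, while a timeline shrinks it, then toggles off its particle effect and briefly delays destruction to let particles fade.
; Overlapping anything except a fireball projectile sends negative heat and positive water.
; That overlap or a blocking hit, which deals no damage, triggers a splash, sound and destruction.
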(event EventBeginPlay
  (Variables|/Script/Engine.MovementComponent|SetVelocity (Variables|Default|GetProjectileMovement1) (Math|Vector|RotateVector (Variables|Default|GetVelocity) (Transformation|GetActorRotation))) ; Set the speed/direction of the projectile
  (Audio|PlaySoundatLocation "/Game/Assets/Audio/WaterWeapon_Fire_Cue.WaterWeapon_Fire_Cue" (Transformation|GetActorLocation) "0, 0, 0" 1.0 1.0) ; Shoot Sound
  (bind _scale (Timeline|LifeSpan Play) ; Timeline blends from 1 to 0.15
    (:Update
      (Transformation|SetActorRelativeScale3D (* (Math|Vector|MakeVector 1.0 1.0 1.0) _scale)) ; Gradually shrink the actor
    )
    (:Finished
      (Components|Activation|ToggleActive (Variables|Default|GetEffect)) ; Turn off effect to give particles a chance to fade instead of disappearing suddenly when the actor is destroyed
      (Utilities|FlowControl|Delay 0.1)
      (Actor|DestroyActor))))

(event Collision|EventActorBeginOverlap
  (params (OtherActor :type Actor%20Object%20Reference))
  (bind _returnvalue (Transformation|GetActorLocation))
  (Utilities|Casting|CastToBP_Projectile_Fireball OtherActor ; Check whether the overlapping actor is another projectile
    (:CastFailed
      (Class|BPIElementalProjectiles|ElementalDamage(Message) OtherActor -0.5 0.5) ; Call this interface function on the target blueprint, if it implements it
      (Effects|SpawnEmitteratLocation "/Game/Assets/Effects/P_Water_Splash.P_Water_Splash" _returnvalue) ; Spawn an impact effect
      (Audio|PlaySoundatLocation "/Game/Assets/Audio/WaterWeapon_Impact_Cue.WaterWeapon_Impact_Cue" _returnvalue "0, 0, 0" 1.0 1.0) ; Water impact sound
      (Actor|DestroyActor))))

(event Collision|EventHit
  (params (MyComp :type Primitive%20Component%20Object%20Reference) (Other :type Actor%20Object%20Reference) (OtherComp :type Primitive%20Component%20Object%20Reference) (bSelfMoved :type Boolean) (HitLocation :type Vector :default "0, 0, 0") (HitNormal :type Vector :default "0, 0, 0") (NormalImpulse :type Vector :default "0, 0, 0") (Hit :type Hit%20Result%20Structure%20%28by%20ref%29))
  (bind _returnvalue (Transformation|GetActorLocation))
  (Effects|SpawnEmitteratLocation "/Game/Assets/Effects/P_Water_Splash.P_Water_Splash" _returnvalue) ; Spawn an impact effect
  (Audio|PlaySoundatLocation "/Game/Assets/Audio/WaterWeapon_Impact_Cue.WaterWeapon_Impact_Cue" _returnvalue "0, 0, 0" 1.0 1.0) ; Water impact sound
  (Actor|DestroyActor))

(fn ConstructionScript)