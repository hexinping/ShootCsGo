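; First-person shooter player character that handles movement, gun use, item pickup and menu hotkeys.
; It creates a launcher and a rifle at start, delegating firing, reloading and ammo-type changes to the current gun, with state checks gating reload and weapon swaps.
; Shoot origin and direction come from the camera and control rotation.
; On death it pulls the camera back and ragdolls a third-person mesh.
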(event Collision|EventActorBeginOverlap
  (params (OtherActor :type Actor%20Object%20Reference)))

(event EventTick
  (params (DeltaSeconds :type Float%20%28single-precision%29)))

(event EventBeginPlay
  (CallFunction|CreateGun "/Game/Blueprints/Launcher.Launcher_C")
  (CallFunction|CreateGun "/Game/Blueprints/Rifle.Rifle_C")
  (Variables|Default|SetCurrentIndex 1)
  (Rendering|SetActorHiddenInGame (CallFunction|GetCurrentGun) false))

(event EventOnDie
  (bind _mesh (Variables|Character|GetMesh))
  (Transformation|AddLocalOffset (Variables|Default|GetCamera) "-400.000000, 0, 0" false false)
  (Class|SkinnedMeshComponent|SetSkeletalMesh _mesh "/Game/Assets/Characters/Models/HeroTPP.HeroTPP" true)
  (Physics|SetSimulatePhysics _mesh true)
  (Collision|SetCollisionEnabled _mesh "QueryAndPhysics"))

(event Input|ActionEvents|InputActionFire
  (params (Key :type Key%20Structure))
  (:Pressed
    (CallFunction|StartFire))
  (:Released
    (CallFunction|EndFire)))

(event Input|ActionEvents|InputActionEquip
  (params (Key :type Key%20Structure))
  (bind _shootgamemode (CallFunction|GetCurrGameMode))
  (bind _fppui (Variables|/Game/Blueprints/ShootGameMode.ShootGameMode_C|GetFppUI _shootgamemode))
  (:Pressed
    (if (not (Variables|/Game/Blueprints/Gun.Gun_C|GetisInReloadBullet (CallFunction|GetCurrentGun)))
      (CallFunction|SwitchWeapon)
      (Default|CallUpdateHpUI _fppui "UpdateBulletNum")
      (Default|CallUpdateHpUI _fppui "UpdateGunIcon"))))

(event Input|AxisEvents|InputAxisMoveForward
  (params (AxisValue :type Float%20%28single-precision%29))
  ;[1 1 1] 沿着人物正向移动
  (Pawn|Input|AddMovementInput (Math|Rotator|GetRotationXVector (Pawn|GetControlRotation :!class /Script/Engine.Pawn)) AxisValue false))

(event Input|AxisEvents|InputAxisLookUp
  (params (AxisValue :type Float%20%28single-precision%29))
  ;[1 1 1] 上下看
  (Pawn|Input|AddControllerPitchInput AxisValue))

(event Input|AxisEvents|InputAxisMoveRight
  (params (AxisValue :type Float%20%28single-precision%29))
  ;[1 1 1] 沿着人物左右移动
  (Pawn|Input|AddMovementInput (Math|Vector|GetRightVector (Pawn|GetControlRotation :!class /Script/Engine.Pawn)) AxisValue false))

(event Input|AxisEvents|InputAxisTurn
  (params (AxisValue :type Float%20%28single-precision%29))
  ;[1 1 1] 朝向
  (Pawn|Input|AddControllerYawInput AxisValue))

(event Input|KeyboardEvents|Tab
  (params (Key :type Key%20Structure))
  (:Pressed
    (bind _returnvalue (UserInterface|CreateWidget "/Game/Blueprints/UI/RankPanel_UI.RankPanel_UI_C"))
    (Variables|Default|SetRankPanelRefence _returnvalue)
    (UserInterface|Viewport|AddtoViewport _returnvalue 0))
  (:Released
    (Widget|RemovefromParent (Variables|Default|GetRankPanelRefence))))

(event Input|KeyboardEvents|K
  (params (Key :type Key%20Structure))
  (bind _gun (CallFunction|GetCurrentGun))
  ;[1 1 1] 换子弹类型
  (:Pressed
    (if (== (Variables|/Game/Blueprints/Gun.Gun_C|GetGunKinds _gun) 1)
      (Default|UpdateBulletIndex _gun))))

(event Input|KeyboardEvents|R
  (params (Key :type Key%20Structure))
  (bind _gun (CallFunction|GetCurrentGun))
  (:Pressed
    ;[1 1 1] 不能连续上子弹
    (if (not (Variables|/Game/Blueprints/Gun.Gun_C|GetisInReloadBullet _gun))
      ;[1 1 1] 开火不能上子弹
      (if (not (Variables|/Game/Blueprints/Gun.Gun_C|GetIsInFire _gun))
        ;[1 1 1] 换枪不能子弹
        (if (not (Variables|Default|GetisInSwitchEquip))
          (if (not (Default|IsFullBullet _gun))
            (Default|PlayerGunReloadAnimatin _gun)))))))

(event Input|KeyboardEvents|B
  (params (Key :type Key%20Structure))
  (:Pressed
    (bind _returnvalue (UserInterface|CreateWidget "/Game/Blueprints/UI/Main_UI.Main_UI_C"))
    (UserInterface|Viewport|AddtoViewport _returnvalue 0)))

(event Input|KeyboardEvents|E
  (params (Key :type Key%20Structure))
  (:Pressed
    (if (Variables|Default|GetisInRange)
      (Default|CallEDPickUPItem))))

(event Input|KeyboardEvents|1
  (params (Key :type Key%20Structure))
  (:Pressed
    (bind _returnvalue (UserInterface|CreateWidget "/Game/Blueprints/UI/Page_UI.Page_UI_C"))
    (UserInterface|Viewport|AddtoViewport _returnvalue 0)
    (CallFunction|ShowUIControl _returnvalue)
    (Variables|Default|SetPageUIRefence _returnvalue)))

(fn ConstructionScript
  (|CallParentFunction))

(fn StartFire
  (Default|StartFire (CallFunction|GetCurrentGun)))

(fn EndFire
  (Default|EndFire (CallFunction|GetCurrentGun)))

(fn SwitchWeapon
  (bind _gun (CallFunction|GetCurrentGun))
  (Variables|Default|SetisInSwitchEquip true)
  (Default|EndFire _gun)
  (Rendering|SetActorHiddenInGame _gun true)
  (Variables|Default|SetCurrentIndex (Math|Integer|%(Integer) (+ (Variables|Default|GetCurrentIndex) 1) (Utilities|Array|Length (Variables|Default|GetGuns))))
  (Rendering|SetActorHiddenInGame (CallFunction|GetCurrentGun) false)
  (Animation|PlayAnimMontage "/Game/Blueprints/Animations/FppEquip_Montage.FppEquip_Montage" 1.0 "None"))

(fn GetShootLocation
  (return (Transformation|GetWorldLocation (Variables|Default|GetCamera))))

(fn GetShootDirection
  (return (Math|Vector|GetForwardVector (Pawn|GetControlRotation :!class /Script/Engine.Pawn))))